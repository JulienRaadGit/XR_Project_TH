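; BP_Guard_Patrol is a guard that walks an endless looping patrol, turning right at timed intervals.
; On BeginPlay it spawns its default controller, prints that controller's name, then starts a delay-driven cycle between MoveForward and RotateRight.
; MoveForward issues a simple move by StepLenth along the facing direction, and RotateRight adds a quarter turn of yaw.
; Tick also nudges the actor forward every frame with a swept, frame-rate-dependent offset.
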(event Custom|MoveForward
  (AI|Navigation|SimpleMovetoLocation (Pawn|GetController) (+ (Transformation|GetActorLocation) (* (Transformation|GetActorForwardVector) (Variables|Default|GetStepLenth))))
  (Utilities|FlowControl|Delay 2.0)
  (CallFunction|RotateRight))

(event Custom|RotateRight
  (bind _returnvalue (Transformation|GetActorRotation))
  (bind (_roll _pitch _yaw) (Math|Rotator|BreakRotator _returnvalue))
  (Transformation|SetActorRotation (Math|Rotator|MakeRotator _roll _pitch (+ _yaw 9e+01)))
  (Utilities|FlowControl|Delay 2.0)
  (CallFunction|MoveForward))

(event EventBeginPlay
  (Pawn|SpawnDefaultController)
  (Utilities|FlowControl|Delay 2.0)
  (Development|PrintString (Utilities|GetDisplayName (Pawn|GetController)))
  (CallFunction|MoveForward))

(event Collision|EventActorBeginOverlap
  (params (OtherActor :type Actor%20Object%20Reference)))

(event EventTick
  (params (DeltaSeconds :type Float%20%28single-precision%29))
  (Transformation|AddActorWorldOffset (* (Transformation|GetActorForwardVector) 2.0) true))

(fn ConstructionScript)