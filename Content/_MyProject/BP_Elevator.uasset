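; BP_Elevator is an elevator actor that runs a timed intro briefing when play begins and then opens its doors.
; BeginPlay chains delays to start instructions on the briefing screen, play an intro speech, wait for it to run, play a ding, then call OpenDoor.
; OpenDoor slides Door1 and Door2 apart simultaneously with eased MoveComponentTo moves.
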(event Custom|OpenDoor
  (Utilities|FlowControl|Sequence
    (:then_0
      (Components|MoveComponentTo (Variables|Default|GetDoor1) (+ (Variables|/Script/Engine.SceneComponent|GetRelativeLocation (Variables|Default|GetDoor1)) "100.000000,0.000000,0.000000") "0, 0, 0" true true 1.0 false))
    (:then_1
      (Components|MoveComponentTo (Variables|Default|GetDoor2) (+ (Variables|/Script/Engine.SceneComponent|GetRelativeLocation (Variables|Default|GetDoor2)) "-100.000000,0.000000,0.000000") "0, 0, 0" true true 1.0 false))))

(event EventBeginPlay
  (Utilities|FlowControl|Delay 2.0)
  (Default|StartInstructions (Variables|Default|GetBriefingScreenRef))
  (Audio|PlaySoundatLocation "/Game/_MyProject/IntroSpeech.IntroSpeech" "0, 0, 0" "0, 0, 0" 1.0 1.0 0.0 0 0 0 0)
  (Utilities|FlowControl|Delay 38.0)
  (Audio|PlaySoundatLocation "/Game/_MyProject/DingElevator.DingElevator" "0, 0, 0" "0, 0, 0" 1.0 1.0 0.0 0 0 0 0)
  (Utilities|FlowControl|Delay 3.0)
  (CallFunction|OpenDoor))

(event Collision|EventActorBeginOverlap
  (params (OtherActor :type Actor%20Object%20Reference)))

(event EventTick
  (params (DeltaSeconds :type Float%20%28single-precision%29)))

(fn ConstructionScript)