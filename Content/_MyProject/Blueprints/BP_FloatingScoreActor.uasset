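; Short-lived actor that displays an animated floating score through a widget component.
; On BeginPlay it turns once to face the player camera, plays the score animation on its WBP_FloatingScore widget, then destroys itself after a brief delay.
; If the widget cast fails, it only prints a debug string and remains in the world.
; The score value is not set in this graph.
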(event EventBeginPlay
  (bind _aswbp_floating_score (Utilities|Casting|CastToWBP_FloatingScore (UserInterface|GetUserWidgetObject (Variables|Default|GetWidget)))
    (:then
      (Transformation|SetActorRotation (Math|Rotator|FindLookatRotation (Transformation|GetActorLocation) (Camera|GetCameraLocation (Game|GetPlayerCameraManager 0))))
      (UserInterface|Animation|PlayAnimation _aswbp_floating_score (Variables|/Game/WBP_FloatingScore.WBP_FloatingScore_C|GetScoreAnim _aswbp_floating_score) 0.0 1 "Forward" 1.0 false)
      (Utilities|FlowControl|Delay 1.0)
      (Actor|DestroyActor))
    (:CastFailed
      (Development|PrintString "Hello"))))

(event Collision|EventActorBeginOverlap
  (params (OtherActor :type Actor%20Object%20Reference)))

(event EventTick
  (params (DeltaSeconds :type Float%20%28single-precision%29)))

(fn ConstructionScript)