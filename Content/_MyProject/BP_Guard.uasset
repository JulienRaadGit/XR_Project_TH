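; BP_Guard is a guard pawn that continuously chases the first player.
; On BeginPlay a looping timer fires every fifth of a second and issues AI MoveTo toward the player pawn.
; Debug prints report its controller, location and the move result.
; An unconnected chain holds an alternative attempt using a spawned default controller and Simple Move To Location.
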(event Custom|CHasePlayer
  (bind _self self)
  (AI|AIMoveTo _self "0, 0, 0" (Game|Player|GetPlayerPawn 0) 5.0 false
    (:then
      (Development|PrintString (Utilities|GetDisplayName (Pawn|GetController _self)))
      (Development|PrintString (Utilities|String|ToString(Vector) (Transformation|GetActorLocation _self))))
    (:OnSuccess
      (Development|PrintString "SUCCESS"))
    (:OnFail
      (Development|PrintString "FAIL"))))

(event EventBeginPlay
  (Utilities|Time|SetTimerbyEvent (delegate Custom|CHasePlayer) 0.2 true))

(fn ConstructionScript)