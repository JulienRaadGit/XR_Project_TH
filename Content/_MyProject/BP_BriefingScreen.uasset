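; BP_BriefingScreen is an in-world screen actor that shows a timed sequence of briefing slides on a plane mesh.
; BeginPlay sets the first slide material on the plane.
; The StartInstructions event then swaps through the remaining five slide materials with fixed delays of several seconds between them, stopping on the last one.
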(event Custom|StartInstructions
  (bind _plane (Variables|Default|GetPlane))
  (Rendering|Material|SetMaterial _plane 0 "/Game/_MyProject/Material/Screen2_Mat.Screen2_Mat")
  (Utilities|FlowControl|Delay 8.0)
  (Rendering|Material|SetMaterial _plane 0 "/Game/_MyProject/Material/Screen3_Mat.Screen3_Mat")
  (Utilities|FlowControl|Delay 7.0)
  (Rendering|Material|SetMaterial _plane 0 "/Game/_MyProject/Material/Screen4_Mat.Screen4_Mat")
  (Utilities|FlowControl|Delay 7.0)
  (Rendering|Material|SetMaterial _plane 0 "/Game/_MyProject/Material/Screen5_Mat.Screen5_Mat")
  (Utilities|FlowControl|Delay 8.0)
  (Rendering|Material|SetMaterial _plane 0 "/Game/_MyProject/Material/Screen6_Mat.Screen6_Mat"))

(event EventBeginPlay
  (Rendering|Material|SetMaterial (Variables|Default|GetPlane) 0 "/Game/_MyProject/Material/Screen1_Mat.Screen1_Mat"))

(event Collision|EventActorBeginOverlap
  (params (OtherActor :type Actor%20Object%20Reference)))

(event EventTick
  (params (DeltaSeconds :type Float%20%28single-precision%29)))

(fn ConstructionScript)